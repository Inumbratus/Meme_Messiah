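; AI controller for the Sanic boss in Level 1, which keeps its focus on the player from BeginPlay.
; The first time AI Perception successfully senses the player, a DoOnce starts the boss behavior tree, caches the possessed Sanic pawn and writes it to the SelfActor blackboard key.
; That same trigger plays a distorted, slowed Green Hill Zone theme as 2D audio.
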(event `self.ReceiveBeginPlay`
  (`self.K2_SetFocus` (`GameplayStatics.GetPlayerCharacter` 0)))

(event `self.AIPerception.OnTargetPerceptionUpdated`
  (params (Actor :type "Actor Object Reference") (Stimulus :type "AIStimulus Structure"))
  (if (and (== (`GameplayStatics.GetPlayerCharacter` 0) Actor) Stimulus_bSuccessfullySensed)
    (`/Engine/EditorBlueprintResources/StandardMacros.DoOnce` false
      (:`Completed`
        (`self.RunBehaviorTree` "/Game/AI/Level1/Sanic/BT_BossAi1_Sanic.BT_BossAi1_Sanic")
        (bind _asbp_boss_ai_1_sanic (cast `/Game/AI/Level1/Sanic/BP_BossAi1_Sanic` (`self.K2_GetPawn`)))
        (bind _output_get (set `self.SanicAiReference` _asbp_boss_ai_1_sanic))
        (`BlackboardComponent.SetValueAsObject` (`AIBlueprintHelperLibrary.GetBlackboard` self) "SelfActor" _output_get)
        (`GameplayStatics.PlaySound2D` "/Game/Audio/Sanic/Green_Hill_Zone_Theme__But_Distorted_and_Slow_Cue.Green_Hill_Zone_Theme__But_Distorted_and_Slow_Cue" 1.0 1.0 0.0 null null)))))

(fn `UserConstructionScript`)