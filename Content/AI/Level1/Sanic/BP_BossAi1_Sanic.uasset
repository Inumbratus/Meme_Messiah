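; BP_BossAi1_Sanic is, by its name and path, the Sanic boss AI character for Level 1, and its graphs hold only debug output.
; Each Tick prints the movement component's yaw rotation rate and the distance to the first player character, with each message lasting one frame.
; The construction script is empty, and no boss behavior is implemented in these graphs.
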(event `self.ReceiveTick`
  (params (DeltaSeconds :type "Float (single-precision)"))
  (bind (_rotationrate_roll _rotationrate_pitch _rotationrate_yaw) (`KismetMathLibrary.BreakRotator` (`CharacterMovementComponent.RotationRate` (`self.CharacterMovement`))))
  (`KismetSystemLibrary.PrintString` (`KismetStringLibrary.Concat_StrStr` (`KismetStringLibrary.Conv_DoubleToString` _rotationrate_yaw) " - Rotation Rate Z") true true (struct :`G` 0.66 :`B` 1.0 :`A` 1.0) DeltaSeconds)
  (`KismetSystemLibrary.PrintString` (`KismetStringLibrary.Concat_StrStr` (`KismetStringLibrary.Conv_DoubleToString` (`self.GetDistanceTo` self (`GameplayStatics.GetPlayerCharacter` 0))) " - Distance to Player") true true (struct :`G` 0.66 :`B` 1.0 :`A` 1.0) (`GameplayStatics.GetWorldDeltaSeconds`)))

(fn `UserConstructionScript`)