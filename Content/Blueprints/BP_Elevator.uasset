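; Elevator actor that carries the player between a bottom and top height when they step into its trigger box.
; Tick closes the door before moving, then reopens it once the cabin stops.
; An enum limits travel to up only, down only or both, with direction flipping at each end.
; Door and cabin share DoorSpeed as a per-frame step, without delta-time scaling.
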(event `self.ReceiveBeginPlay`
  (bind _asfirst_person_character (cast `/Game/FirstPersonBP/Blueprints/FirstPersonCharacter` (`GameplayStatics.GetPlayerPawn` 0)))
  (set `self.PlayerPawn` _asfirst_person_character)
  (switch `/Game/Blueprints/ElevatorEnum` (`self.ElevatorMovement`)
    (:`NewEnumerator0`
      (set `self.MovingUp` true))
    (:`NewEnumerator1`
      (set `self.MovingUp` false))))

(event `self.ReceiveTick`
  (params (DeltaSeconds :type "Float (single-precision)"))
  (bind _elevatormovement (`self.ElevatorMovement`))
  (if (`self.IsMoving`)
    (bind _isclosed (`self.CloseDoor`))
    (if _isclosed
      (if (`self.MovingUp`)
        (switch `/Game/Blueprints/ElevatorEnum` _elevatormovement
          (:`NewEnumerator0`
            (`self.GoUp` :!label _label))
          (:`NewEnumerator1`
            (set `self.MovingUp` false))
          (:`NewEnumerator2`
            (goto _label)))
        (else
          (switch `/Game/Blueprints/ElevatorEnum` _elevatormovement
            (:`NewEnumerator0`
              (set `self.MovingUp` true))
            (:`NewEnumerator1`
              (`self.GoDown` :!label _label_2))
            (:`NewEnumerator2`
              (goto _label_2))))))
    (else
      (`self.OpenDoor`))))

(event `self.Box.OnComponentBeginOverlap`
  (params (OverlappedComponent :type "PrimitiveComponent Object Reference") (OtherActor :type "Actor Object Reference") (OtherComp :type "PrimitiveComponent Object Reference") (OtherBodyIndex :type Integer) (bFromSweep :type Boolean) (SweepResult :type "HitResult Structure (by ref)"))
  (if (and (== OtherActor (`self.PlayerPawn`)) (not (`self.IsMoving`)))
    (set `self.IsMoving` true)))

(fn `CloseDoor`
  (returns (IsClosed :type Boolean))
  (bind (_relativelocation_x _relativelocation_y _relativelocation_z) (`KismetMathLibrary.BreakVector` (`SceneComponent.RelativeLocation` (`self.Door`))))
  (if (> _relativelocation_z 115.0)
    (`SceneComponent.K2_AddRelativeLocation` (`self.Door`) (`KismetMathLibrary.MakeVector` 0.0 0.0 (* (`self.DoorSpeed`) -1.0)) false false)
    (return false)
    (else
      (return true))))

(fn `GoDown`
  (bind (_returnvalue_x _returnvalue_y _returnvalue_z) (`KismetMathLibrary.BreakVector` (`self.K2_GetActorLocation`)))
  (if (> _returnvalue_z (`self.BottomZPos`))
    (`self.K2_SetActorLocation` (`KismetMathLibrary.MakeVector` _returnvalue_x _returnvalue_y (+ _returnvalue_z (* (`self.DoorSpeed`) -1.0))))
    (else
      (set `self.IsMoving` false)
      (set `self.MovingUp` true))))

(fn `GoUp`
  (bind (_returnvalue_x _returnvalue_y _returnvalue_z) (`KismetMathLibrary.BreakVector` (`self.K2_GetActorLocation`)))
  (if (< _returnvalue_z (`self.TopZPos`))
    (`self.K2_SetActorLocation` (`KismetMathLibrary.MakeVector` _returnvalue_x _returnvalue_y (+ _returnvalue_z (`self.DoorSpeed`))))
    (else
      (set `self.IsMoving` false)
      (set `self.MovingUp` false))))

(fn `OpenDoor`
  (bind (_relativelocation_x _relativelocation_y _relativelocation_z) (`KismetMathLibrary.BreakVector` (`SceneComponent.RelativeLocation` (`self.Door`))))
  (if (< _relativelocation_z 325.0)
    (`SceneComponent.K2_AddRelativeLocation` (`self.Door`) (`KismetMathLibrary.MakeVector` 0.0 0.0 (`self.DoorSpeed`)) false false)))

(fn `UserConstructionScript`)