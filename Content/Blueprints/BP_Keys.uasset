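; A collectible colour key pickup that grants the player a door key when touched.
; A KeyColours enum picks the billboard sprite in the construction script for editor preview, and again at BeginPlay along with a matching point light colour and slot index.
; On box overlap with FirstPersonCharacter, it sets that index in the character's DoorKeys array to true and destroys itself.
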(event `self.ReceiveBeginPlay`
  (bind _pointlight (`self.PointLight`))
  (bind _billboard (`self.Billboard`))
  (switch `/Game/Blueprints/KeysEnum` (`self.KeyColours`)
    (:`NewEnumerator0`
      (`BillboardComponent.SetSprite` _billboard "/Game/Assets/Images/BlueKey.BlueKey")
      (set `self.keyint` 0)
      (`LightComponent.SetLightColor` _pointlight (struct :`B` 1.0 :`A` 1.0) true))
    (:`NewEnumerator1`
      (`BillboardComponent.SetSprite` _billboard "/Game/Assets/Images/YellowKey.YellowKey")
      (set `self.keyint` 1)
      (`LightComponent.SetLightColor` _pointlight (struct :`R` 1.0 :`G` 1.0 :`A` 1.0) true))
    (:`NewEnumerator2`
      (`BillboardComponent.SetSprite` _billboard "/Game/Assets/Images/RedKey.RedKey")
      (set `self.keyint` 2)
      (`LightComponent.SetLightColor` _pointlight (struct :`R` 1.0 :`A` 1.0) true))))

(event `self.Box.OnComponentBeginOverlap`
  (params (OverlappedComponent :type "PrimitiveComponent Object Reference") (OtherActor :type "Actor Object Reference") (OtherComp :type "PrimitiveComponent Object Reference") (OtherBodyIndex :type Integer) (bFromSweep :type Boolean) (SweepResult :type "HitResult Structure (by ref)"))
  (bind _asfirst_person_character (cast `/Game/FirstPersonBP/Blueprints/FirstPersonCharacter` OtherActor))
  (`KismetArrayLibrary.Array_Set` (`/Game/FirstPersonBP/Blueprints/FirstPersonCharacter.DoorKeys` _asfirst_person_character) (`self.keyint`) true)
  (`self.K2_DestroyActor`))

(fn `UserConstructionScript`
  (bind _billboard (`self.Billboard`))
  (switch `/Game/Blueprints/KeysEnum` (`self.KeyColours`)
    (:`NewEnumerator0`
      (`BillboardComponent.SetSprite` _billboard "/Game/Assets/Images/BlueKey.BlueKey"))
    (:`NewEnumerator1`
      (`BillboardComponent.SetSprite` _billboard "/Game/Assets/Images/YellowKey.YellowKey"))
    (:`NewEnumerator2`
      (`BillboardComponent.SetSprite` _billboard "/Game/Assets/Images/RedKey.RedKey"))))