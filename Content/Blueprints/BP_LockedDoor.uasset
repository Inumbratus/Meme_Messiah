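; A colour-keyed locked door that unlocks when the first-person player enters its trigger box holding the matching key.
; DoorColour tints two point lights in the construction script and at BeginPlay, which also maps it to an index into the player's DoorKeys array.
; Unlocking turns the lights green and persists.
; Tick then slides the Cube up while the player overlaps the box and back down otherwise, within fixed height limits.
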(event `self.ReceiveBeginPlay`
  (bind _pointlight (`self.PointLight`))
  (bind _asfirst_person_character (cast `/Game/FirstPersonBP/Blueprints/FirstPersonCharacter` (`GameplayStatics.GetPlayerPawn` 0)))
  (set `self.PlayerPawn` _asfirst_person_character)
  (switch `/Game/Blueprints/KeysEnum` (`self.DoorColour`)
    (:`NewEnumerator0`
      (`LightComponent.SetLightColor` _pointlight (struct :`G` 0.405744 :`B` 1.0 :`A` 1.0) true)
      (`LightComponent.SetLightColor` (`self.PointLight1`) (struct :`G` 0.405744 :`B` 1.0 :`A` 1.0) true)
      (set `self.doorint` 0))
    (:`NewEnumerator1`
      (`LightComponent.SetLightColor` _pointlight (struct :`R` 1.0 :`G` 0.899544 :`A` 1.0) true)
      (`LightComponent.SetLightColor` (`self.PointLight1`) (struct :`R` 1.0 :`G` 0.899544 :`A` 1.0) true)
      (set `self.doorint` 1))
    (:`NewEnumerator2`
      (`LightComponent.SetLightColor` _pointlight (struct :`R` 1.0 :`A` 1.0) true)
      (`LightComponent.SetLightColor` (`self.PointLight1`) (struct :`R` 1.0 :`A` 1.0) true)
      (set `self.doorint` 2))))

(event `self.Box.OnComponentBeginOverlap`
  (params (OverlappedComponent :type "PrimitiveComponent Object Reference") (OtherActor :type "Actor Object Reference") (OtherComp :type "PrimitiveComponent Object Reference") (OtherBodyIndex :type Integer) (bFromSweep :type Boolean) (SweepResult :type "HitResult Structure (by ref)"))
  (bind _playerpawn (`self.PlayerPawn`))
  (if (and (== OtherActor _playerpawn) (`|GetArrayItem` (`/Game/FirstPersonBP/Blueprints/FirstPersonCharacter.DoorKeys` _playerpawn) (`self.doorint`)))
    (set `self.unlocked` true)
    (`LightComponent.SetLightColor` (`self.PointLight1`) (struct :`R` 0.040347 :`G` 1.0 :`B` 0.038727 :`A` 1.0) true)
    (`LightComponent.SetLightColor` (`self.PointLight`) (struct :`R` 0.040347 :`G` 1.0 :`B` 0.038727 :`A` 1.0) true)))

(event `self.ReceiveTick`
  (params (DeltaSeconds :type "Float (single-precision)"))
  (if (and (`PrimitiveComponent.IsOverlappingActor` (`self.Box`) (`self.PlayerPawn`)) (`self.unlocked`))
    (`self.OpenDoor`)
    (else
      (`self.CloseDoor`))))

(fn `CloseDoor`
  (bind (_relativelocation_x _relativelocation_y _relativelocation_z) (`KismetMathLibrary.BreakVector` (`SceneComponent.RelativeLocation` (`self.Cube`))))
  (if (> _relativelocation_z 130.0)
    (`SceneComponent.K2_AddRelativeLocation` (`self.Cube`) (`KismetMathLibrary.MakeVector` 0.0 0.0 (* (`self.Speed`) -1.0)) false false)))

(fn `OpenDoor`
  (bind (_relativelocation_x _relativelocation_y _relativelocation_z) (`KismetMathLibrary.BreakVector` (`SceneComponent.RelativeLocation` (`self.Cube`))))
  (if (< _relativelocation_z 370.0)
    (`SceneComponent.K2_AddRelativeLocation` (`self.Cube`) (`KismetMathLibrary.MakeVector` 0.0 0.0 (`self.Speed`)) false false)))

(fn `UserConstructionScript`
  (bind _pointlight (`self.PointLight`))
  (switch `/Game/Blueprints/KeysEnum` (`self.DoorColour`)
    (:`NewEnumerator0`
      (`LightComponent.SetLightColor` _pointlight (struct :`G` 0.405744 :`B` 1.0 :`A` 1.0) true)
      (`LightComponent.SetLightColor` (`self.PointLight1`) (struct :`G` 0.405744 :`B` 1.0 :`A` 1.0) true))
    (:`NewEnumerator1`
      (`LightComponent.SetLightColor` _pointlight (struct :`R` 1.0 :`G` 0.899544 :`A` 1.0) true)
      (`LightComponent.SetLightColor` (`self.PointLight1`) (struct :`R` 1.0 :`G` 0.899544 :`A` 1.0) true))
    (:`NewEnumerator2`
      (`LightComponent.SetLightColor` _pointlight (struct :`R` 1.0 :`A` 1.0) true)
      (`LightComponent.SetLightColor` (`self.PointLight1`) (struct :`R` 1.0 :`A` 1.0) true))))