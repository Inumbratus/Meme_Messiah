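; Colour-coded locked door that unlocks permanently when the player enters its trigger box with the matching key, or starts unlocked if it needs no key.
; The construction script sets the door material from DoorColour, and BeginPlay maps that colour to an index into the player's DoorKeys.
; Tick raises the door while the player or a DebugEnemy overlaps an unlocked door, otherwise lowers it, using paired gates to play one sound per change.
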(event `self.ReceiveBeginPlay`
  (bind _asfirst_person_character (cast `/Game/FirstPersonBP/Blueprints/FirstPersonCharacter` (`GameplayStatics.GetPlayerPawn` 0)))
  (set `self.PlayerPawn` _asfirst_person_character)
  (switch `/Game/Blueprints/KeysEnum` (`self.DoorColour`)
    (:`NewEnumerator3`
      (set `self.unlocked` true))
    (:`NewEnumerator0`
      (set `self.doorint` 0))
    (:`NewEnumerator1`
      (set `self.doorint` 1))
    (:`NewEnumerator2`
      (set `self.doorint` 2))))

(event `self.Box.OnComponentBeginOverlap`
  (params (OverlappedComponent :type "PrimitiveComponent Object Reference") (OtherActor :type "Actor Object Reference") (OtherComp :type "PrimitiveComponent Object Reference") (OtherBodyIndex :type Integer) (bFromSweep :type Boolean) (SweepResult :type "HitResult Structure (by ref)"))
  (bind _playerpawn (`self.PlayerPawn`))
  (if (and (== OtherActor _playerpawn) (`|GetArrayItem` (`/Game/FirstPersonBP/Blueprints/FirstPersonCharacter.DoorKeys` _playerpawn) (`self.doorint`)))
    (set `self.unlocked` true)))

(event `self.ReceiveTick`
  (params (DeltaSeconds :type "Float (single-precision)"))
  (bind _unlocked (`self.unlocked`))
  (if (or (and (`PrimitiveComponent.IsOverlappingActor` (`self.Box`) (`self.PlayerPawn`)) _unlocked) (and _unlocked (> (`KismetArrayLibrary.Array_Length` (`PrimitiveComponent.GetOverlappingActors` (`self.Box`) "/Game/FirstPersonBP/Blueprints/DebugEnemy.DebugEnemy_C")) 0)))
    (`self.OpenDoor`)
    (`|ExecutionSequence`
      (:`then_0`
        (`/Engine/EditorBlueprintResources/StandardMacros.Gate` true :!label _label
          (:`Exit`
            _)))
      (:`then_1`
        (goto _label :!via `Close`))
      (:`then_2`
        (goto _label_2 :!via `Open`)))
    (else
      (`self.CloseDoor`)
      (`|ExecutionSequence`
        (:`then_0`
          (`/Engine/EditorBlueprintResources/StandardMacros.Gate` true :!label _label_2
            (:`Exit`
              _)))
        (:`then_1`
          (goto _label_2 :!via `Close`))
        (:`then_2`
          (goto _label :!via `Open`)))))
  (`GameplayStatics.PlaySoundAtLocation` "/Game/Audio/door_sound.door_sound" (`SceneComponent.K2_GetComponentLocation` (`self.Cube`)) (struct) 0.5 1.0 0.0 null null null))

(fn `CloseDoor`
  (bind (_relativelocation_x _relativelocation_y _relativelocation_z) (`KismetMathLibrary.BreakVector` (`SceneComponent.RelativeLocation` (`self.Cube`))))
  (if (> _relativelocation_z 130.0)
    (`SceneComponent.K2_AddRelativeLocation` (`self.Cube`) (`KismetMathLibrary.MakeVector` 0.0 0.0 (* (`self.Speed`) -1.0)) false false)))

(fn `OpenDoor`
  (bind (_relativelocation_x _relativelocation_y _relativelocation_z) (`KismetMathLibrary.BreakVector` (`SceneComponent.RelativeLocation` (`self.Cube`))))
  (if (< _relativelocation_z 370.0)
    (`SceneComponent.K2_AddRelativeLocation` (`self.Cube`) (`KismetMathLibrary.MakeVector` 0.0 0.0 (`self.Speed`)) false false)))

(fn `UserConstructionScript`
  (bind _cube (`self.Cube`))
  (switch `/Game/Blueprints/KeysEnum` (`self.DoorColour`)
    (:`NewEnumerator3`
      (`PrimitiveComponent.SetMaterial` _cube 0 "/Game/FirstPersonBP/Blueprints/KeyDoorMaterialGreen.KeyDoorMaterialGreen"))
    (:`NewEnumerator0`
      (`PrimitiveComponent.SetMaterial` _cube 0 "/Game/FirstPersonBP/Blueprints/KeyDoorMaterialPointerMaterialBlue.KeyDoorMaterialPointerMaterialBlue"))
    (:`NewEnumerator1`
      (`PrimitiveComponent.SetMaterial` _cube 0 "/Game/FirstPersonBP/Blueprints/KeyDoorMaterialPointerMaterialYellow.KeyDoorMaterialPointerMaterialYellow"))
    (:`NewEnumerator2`
      (`PrimitiveComponent.SetMaterial` _cube 0 "/Game/FirstPersonBP/Blueprints/KeyDoorMaterialPointerMaterialRed.KeyDoorMaterialPointerMaterialRed"))))