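; Second boss AI actor that becomes active when the player comes within range, then throws knives.
; BeginPlay caches the player character; Tick checks distance until activation, then spawns BP_knife at the Billboard's transform, paced by a Delay.
; The stage-one health check compares Health to itself divided by one, so it always passes.
; Gordan sprite swaps are present but unconnected, and no later stages are implemented.
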(event `self.ReceiveBeginPlay`
  (bind _asfirst_person_character (cast `/Game/FirstPersonBP/Blueprints/FirstPersonCharacter` (`GameplayStatics.GetPlayerCharacter` 0)))
  (set `self.Player` _asfirst_person_character))

(event `self.ReceiveTick`
  (params (DeltaSeconds :type "Float (single-precision)"))
  (bind _health (`self.Health`))
  (if (`self.Active`)
    (if (not (< _health (/ _health 1.0)))
      ;[1 1 1] Stage 1
      (`KismetSystemLibrary.Delay` 2.0)
      (`|SpawnActorFromClass` "/Game/Blueprints/BP_knife.BP_knife_C" (`SceneComponent.K2_GetComponentToWorld` (`self.Billboard`)) "Undefined" "OverrideRootScale" null null))
    (else
      (set `self.Active` (< (`KismetMathLibrary.Vector_Distance` (`self.K2_GetActorLocation`) (`self.K2_GetActorLocation` (`self.Player`))) 1000.0)))))

(fn `UserConstructionScript`)