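; A key pickup actor that gives the first-person player one of three coloured door keys.
; The KeyColours enum sets the billboard sprite in the construction script for editor preview and again on BeginPlay, which also maps the colour to an array index.
; When a FirstPersonCharacter overlaps the box, it sets that index in the character's DoorKeys array to true and destroys itself.
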(event `self.ReceiveBeginPlay`
  (bind _billboard (`self.Billboard`))
  (switch `/Game/Blueprints/KeysEnum` (`self.KeyColours`)
    (:`NewEnumerator0`
      (`BillboardComponent.SetSprite` _billboard "/Game/Assets/Images/BlueKey.BlueKey")
      (set `self.keyint` 0))
    (:`NewEnumerator1`
      (`BillboardComponent.SetSprite` _billboard "/Game/Assets/Images/YellowKey.YellowKey")
      (set `self.keyint` 1))
    (:`NewEnumerator2`
      (`BillboardComponent.SetSprite` _billboard "/Game/Assets/Images/RedKey.RedKey")
      (set `self.keyint` 2))))

(event `self.Box.OnComponentBeginOverlap`
  (params (OverlappedComponent :type "PrimitiveComponent Object Reference") (OtherActor :type "Actor Object Reference") (OtherComp :type "PrimitiveComponent Object Reference") (OtherBodyIndex :type Integer) (bFromSweep :type Boolean) (SweepResult :type "HitResult Structure (by ref)"))
  (bind _asfirst_person_character (cast `/Game/FirstPersonBP/Blueprints/FirstPersonCharacter` OtherActor))
  (`KismetArrayLibrary.Array_Set` (`/Game/FirstPersonBP/Blueprints/FirstPersonCharacter.DoorKeys` _asfirst_person_character) (`self.keyint`) true)
  (`self.K2_DestroyActor`))

(fn `UserConstructionScript`
  (bind _billboard (`self.Billboard`))
  (switch `/Game/Blueprints/KeysEnum` (`self.KeyColours`)
    (:`NewEnumerator0`
      (`BillboardComponent.SetSprite` _billboard "/Game/Assets/Images/BlueKey.BlueKey"))
    (:`NewEnumerator1`
      (`BillboardComponent.SetSprite` _billboard "/Game/Assets/Images/YellowKey.YellowKey"))
    (:`NewEnumerator2`
      (`BillboardComponent.SetSprite` _billboard "/Game/Assets/Images/RedKey.RedKey"))))